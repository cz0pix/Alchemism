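; BP_Piwnica is a cellar ("piwnica") door or hatch that opens and sends the player to the Alchemism level.
; PiwnicaOpen plays a Timeline that lerps the Piwnica component from the rotation saved at BeginPlay to OpenRotator.
; The same Update pin chains delays, a WDG_fadein widget animation and the level load, rather than waiting for Finished.
; Camera-fade and level-sequence fade nodes remain unconnected.
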(event Custom|Piwnica%20Open
  (bind _newtrack_2 (Timeline|Timeline Play)
    (:Update
      (Transformation|SetRelativeRotation (Variables|Default|GetPiwnica) (Math|Rotator|Lerp(Rotator) (stale EventBeginPlay _output_get) (Variables|Default|GetOpenRotator) _newtrack_2) false false)
      (Utilities|FlowControl|Delay 2.0)
      (bind _returnvalue (UserInterface|CreateWidget "/Game/piwnica_teleport/fadein/WDG_fadein.WDG_fadein_C"))
      (UserInterface|Viewport|AddtoViewport _returnvalue 0)
      (UserInterface|Animation|PlayAnimation _returnvalue (Variables|/Game/piwnica_teleport/fadein/WDG_fadein.WDG_fadein_C|GetFadein1 _returnvalue) 0.0 1 "Forward" 1.0 false)
      (Utilities|FlowControl|Delay 2.0)
      (Game|OpenLevel(byName) "Alchemism"))))

(event EventBeginPlay
  (bind _output_get (Variables|Default|SetCloseRotation (Variables|/Script/Engine.SceneComponent|GetRelativeRotation (Variables|Default|GetPiwnica)))))

(fn ConstructionScript)