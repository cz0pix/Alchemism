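; BP_Piwnica1 is a cellar (piwnica) opening that swings open and then teleports the player.
; PiwnicaOpen1 runs a timeline that rotates the Piwnica component from its BeginPlay rotation to OpenRotator.
; Shortly after it finishes, the player pawn teleports to TeleportTarget2 with zero rotation, and Piwnica snaps to zero relative rotation.
; A fade-in widget sequence is present but disconnected, so it never runs.
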(event Custom|Piwnica%20Open1
  (bind _newtrack_2 (Timeline|Timeline Play)
    (:Update
      (Transformation|SetRelativeRotation (Variables|Default|GetPiwnica) (Math|Rotator|Lerp(Rotator) (stale EventBeginPlay _output_get) (Variables|Default|GetOpenRotator) _newtrack_2) false false))
    (:Finished
      (Utilities|FlowControl|Delay 0.1)
      (Transformation|Teleport (Game|Player|GetPlayerPawn 0) (Transformation|GetActorLocation (Variables|Default|GetTeleportTarget2)) "0, 0, 0")
      (Transformation|SetRelativeRotation (Variables|Default|GetPiwnica) "0, 0, 0" false false))))

(event EventBeginPlay
  (bind _output_get (Variables|Default|SetCloseRotation (Variables|/Script/Engine.SceneComponent|GetRelativeRotation (Variables|Default|GetPiwnica)))))

(fn ConstructionScript)