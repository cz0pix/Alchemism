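; BP_Dzwig is a VR lever that the player grabs and rotates to trigger opening of the cellar (BP_Piwnica), found at BeginPlay.
; While held, a looping timer runs UpdateRotation, turning the motion controller's relative Y offset into clamped lever roll.
; Past a roll threshold it calls PiwnicaOpen on each tick of that timer.
; Author notes say the intended cellar rotation and level opening do not work yet.
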(event OnGrabbed(GrabComponent)
  (params (Motion%20Controller :type Motion%20Controller%20Component%20Object%20Reference))
  ;[0.15 0.15 0.15 0.5] This part works
  (Variables|Default|SetMotion%20Controller Motion%20Controller)
  (bind _returnvalue (Utilities|Time|SetTimerbyFunctionName 0 "UpdateRotation" 0.02 true))
  (Variables|Default|SetTimer _returnvalue))

(event OnDropped(GrabComponent)
  ;[0.15 0.15 0.15 0.5] This part works
  (Utilities|Time|ClearandInvalidateTimerbyHandle (Variables|Default|GetTimer))
  (Variables|Default|SetMotion%20Controller 0))

(event EventBeginPlay
  ;[0.15 0.15 0.15 0.5] This part works
  (bind _returnvalue (Actor|GetActorOfClass "/Game/piwnica_teleport/BP_Piwnica.BP_Piwnica_C"))
  (Variables|Default|SetPiwnicaRef _returnvalue))

(fn ConstructionScript)

(fn UpdateRotation
  (bind _grabcomponent (Variables|Default|GetGrabComponent))
  (bind _motion_controller (Variables|Default|GetMotion%20Controller))
  (bind _dzwig (Variables|Default|GetDzwig))
  (bind _returnvalue (Transformation|GetWorldTransform _motion_controller))
  (bind _returnvalue_2 (Transformation|GetWorldTransform _grabcomponent))
  (bind _relativelocation (Variables|/Script/Engine.SceneComponent|GetRelativeLocation _grabcomponent))
  (bind _relativerotation (Variables|/Script/Engine.SceneComponent|GetRelativeRotation _dzwig))
  (bind _returnvalue_3 (Math|Transform|MakeRelativeTransform _returnvalue _returnvalue_2))
  (bind _returnvalue_4 (- _relativelocation (.location _returnvalue_3)))
  (bind _returnvalue_5 (+ (.roll _relativerotation) (.y _returnvalue_4)))
  (bind _returnvalue_6 (Math|Float|Clamp(Float) _returnvalue_5 0.0 4e+01))
  ;[0.15 0.15 0.15 0.5] This part works and moves dzwig
  (Transformation|SetRelativeRotation _dzwig (Math|Rotator|MakeRotator _returnvalue_6 (.pitch _relativerotation) (.yaw _relativerotation)) false false)
  ;[0.15 0.15 0.15 0.5] This is supposed to rotate the piwnica and open new level but it doesn't work
  (if (> _returnvalue_6 3e+01)
    (Default|PiwnicaOpen (Variables|Default|GetPiwnicaRef))))