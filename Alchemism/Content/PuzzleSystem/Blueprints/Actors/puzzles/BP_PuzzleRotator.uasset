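; Puzzle piece actor that, once placed, turns in quarter steps until it reaches its target orientation.
; OnPlaced freezes physics and sets query-only collision, enabling OnRotate, which plays a click and lerps the mesh 90 degrees on a timeline.
; Each finished turn advances RotateIndex; a TargetIndex match locks the piece, plays a success sound and notifies PuzzleManager.
; The wrap to zero after four turns skips that match check.
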(event EventBeginPlay)

(event Collision|EventActorBeginOverlap
  (params (OtherActor :type Actor%20Object%20Reference)))

(event EventTick
  (params (DeltaSeconds :type Float%20%28single-precision%29)))

(event EventOnRotate
  (if (Variables|Default|GetIsPlaced)
    (if (not (Variables|Default|Getis%20solved))
      (if (not (Audio|Components|Audio|IsPlaying (Variables|Default|GetTL_timeline)))
        (Audio|PlaySoundatLocation "/Engine/VREditor/Sounds/UI/Click_on_Button.Click_on_Button" (Transformation|GetActorLocation) "0, 0, 0" 1.0 1.0 0.0 0 0 0 0)
        (bind _al_ha (Timeline|TL_timeline PlayFromStart)
          (:Update
            (Transformation|SetRelativeRotation (Variables|Default|Getpuzzle_piece) (Math|Rotator|MakeRotator 0.0 (Math|Float|Lerp (.pitch (Variables|Default|GetPieceRotation)) (- (.pitch (Variables|Default|GetPieceRotation)) 9e+01) _al_ha) 0.0) false false))
          (:Finished
            (Variables|Default|SetPieceRotation (Math|Rotator|MakeRotator 0.0 (Math|Float|Lerp (.pitch (Variables|Default|GetPieceRotation)) (- (.pitch (Variables|Default|GetPieceRotation)) 9e+01) _al_ha) 0.0))
            (bind _result (Math|Integer|IncrementInt (Variables|Default|GetRotateIndex))
              (:%20%20
                (bind _output_get (Variables|Default|SetRotateIndex _result))
                (if (>= _output_get 4)
                  (Variables|Default|SetRotateIndex 0)
                  (elif (== (Variables|Default|GetTargetIndex) (Variables|Default|GetRotateIndex))
                    (Development|PrintString "correct" true true "(R=0.245093,G=1.000000,B=0.223487,A=1.000000)")
                    (Variables|Default|Setis%20solved true)
                    (Audio|PlaySound2D "/Engine/EditorSounds/Notifications/CompileSuccess.CompileSuccess" 1.0 1.0 0.0 0 0)
                    (Class|BPIPuzzle|OnPuzzleComplete(Message) (Variables|Default|GetPuzzleManager))
                    (else
                      (Development|PrintString "not correct" true true "(R=0.432292,G=0.033577,B=0.057536,A=1.000000)"))))))))))))

(fn ConstructionScript
  (Components|StaticMesh|SetStaticMesh (Variables|Default|Getpuzzle_piece) (Variables|Default|GetPuzzle%20piece%20mesh)))

(fn OnPlaced
  (Variables|Default|SetIsPlaced true)
  ;[0.15 0.15 0.15 0.5] prevent wobbling after placed
  (Physics|SetSimulatePhysics (Variables|Default|Getpuzzle_piece) false)
  (Physics|SetPhysicsLinearVelocity (Variables|Default|Getpuzzle_piece) "0, 0, 0" false "None")
  (Class|PrimitiveComponent|SetPhysicsAngularVelocityinDegrees (Variables|Default|Getpuzzle_piece) "0, 0, 0" false "None")
  (Collision|SetCollisionEnabled (Variables|Default|Getpuzzle_piece) "QueryOnly"))

(fn GetData
  (return))