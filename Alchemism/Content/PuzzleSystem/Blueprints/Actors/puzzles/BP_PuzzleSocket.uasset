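; BP_PuzzleSocket is a puzzle socket actor that snaps rotator puzzle pieces into place.
; When a BP_PuzzleRotator overlaps SnapZone, it moves to SnapPoint's location and rotation, gets flagged as placed and has OnPlaced called.
; It then becomes the VR pawn's CurrentPuzzlePiece.
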(event OnComponentBeginOverlap(snapzone)
  (params (OverlappedComponent :type Primitive%20Component%20Object%20Reference) (OtherActor :type Actor%20Object%20Reference) (OtherComp :type Primitive%20Component%20Object%20Reference) (OtherBodyIndex :type Integer) (bFromSweep :type Boolean) (SweepResult :type Hit%20Result%20Structure%20%28by%20ref%29))
  (bind _asbp_puzzle_rotator (Utilities|Casting|CastToBP_PuzzleRotator OtherActor))
  (Transformation|SetActorLocationAndRotation _asbp_puzzle_rotator (Transformation|GetWorldLocation (Variables|Default|Getsnap%20point)) (Transformation|GetWorldRotation (Variables|Default|Getsnap%20point)))
  (Variables|/Game/PuzzleSystem/Blueprints/Actors/puzzles/BP_PuzzleRotator.BP_PuzzleRotator_C|SetIsPlaced _asbp_puzzle_rotator true)
  (Default|OnPlaced _asbp_puzzle_rotator)
  (bind _asvrpawn (Utilities|Casting|CastToVRPawn (Game|Player|GetPlayerPawn 0)))
  (Variables|/Game/VRTemplate/Blueprints/VRPawn.VRPawn_C|SetCurrentPuzzlePiece _asvrpawn _asbp_puzzle_rotator))

(event EventBeginPlay)

(event Collision|EventActorBeginOverlap
  (params (OtherActor :type Actor%20Object%20Reference)))

(event EventTick
  (params (DeltaSeconds :type Float%20%28single-precision%29)))

(fn ConstructionScript)