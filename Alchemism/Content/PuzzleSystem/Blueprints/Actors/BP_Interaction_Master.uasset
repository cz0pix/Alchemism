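; BP_Interaction_Master is a base interaction actor in the puzzle system, with a static mesh and a collision sphere.
; Its construction script applies the mesh, world scale and relative location from a MeshSettings struct.
; A positive CustomCollisionRadius overrides the sphere's radius.
; GetData is an empty stub.
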(fn ConstructionScript
  (bind _meshsettings (Utilities|Struct|Break))
  (Components|StaticMesh|SetStaticMesh (Variables|Default|GetStaticMesh) (.staticmesh _meshsettings))
  (Transformation|SetWorldScale3D (Variables|Default|GetStaticMesh) (.itemsize _meshsettings))
  (Transformation|SetRelativeLocation (Variables|Default|GetStaticMesh) (.itemlocation _meshsettings) false false)
  (if (> (Variables|Default|GetCustomCollisionRadius) 0.0)
    (Components|Sphere|SetSphereRadius (Variables|Default|GetSphere) (Variables|Default|GetCustomCollisionRadius) true)))

(fn GetData
  (return))