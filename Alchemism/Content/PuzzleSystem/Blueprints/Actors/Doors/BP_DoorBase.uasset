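; Base interactable hinged door for the puzzle system that swings open and closed, with optional key locking.
; On interact, a locked door searches the save manager's keys for its KeyID, toggling if found, otherwise playing a locked sound and timeline-driven rattle.
; A timeline lerps mesh yaw, playing forward or reversed with matching sounds, and Invert flips the swing direction.
; The construction script poses the mesh from its initial closed state.
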(event Custom|DoorState
  ;[0 0 0] Door Logic
  (if (Variables|DoorSettings|Custom|GetIsClosed?)
    (Variables|DoorSettings|Custom|SetIsClosed? false)
    (CallFunction|DoorOpenSound)
    (bind _alpha (Timeline|TL_Door PlayFromStart)
      (:Update
        (Transformation|SetRelativeRotation (Variables|Default|GetStaticMesh) (Math|Rotator|MakeRotator 0.0 0.0 (Math|Float|Lerp 0.0 (select (Variables|DoorSettings|Custom|GetInvert) -85.0 85.0) _alpha)) false false)))
    (else
      (Variables|DoorSettings|Custom|SetIsClosed? true)
      (CallFunction|DoorCloseSound)
      (Timeline|TL_Door ReverseFromEnd))))

(event Custom|DoorOpenSound
  ;[0 0 0] Sound Logic
  ;;[0 0 0] Opening Sound Logic
  (Audio|PlaySoundatLocation (Variables|DoorSettings|Sounds|GetOpenSound) (Variables|Default|GetDoorSoundLocation) "0, 0, 0" 1.0 1.0 0.0 0 0 0 0))

(event Custom|DoorCloseSound
  ;[0 0 0] Sound Logic
  ;;[0 0 0] Opening Sound Logic
  (Utilities|FlowControl|Delay 0.5)
  (Audio|PlaySoundatLocation (Variables|DoorSettings|Sounds|GetCloseSound) (Variables|Default|GetDoorSoundLocation) "0, 0, 0" 1.0 1.0 0.0 0 0 0 0))

(event Custom|ForceToOpen
  ;[0 0 0] Sound Logic
  ;;[0 0 0] Opening Sound Logic
  (Audio|PlaySoundatLocation (Variables|DoorSettings|Sounds|GetLockedSound) (Variables|Default|GetDoorSoundLocation) "0, 0, 0" 1.0 1.0 0.0 0 0 0 0))

(event EventBeginPlay
  ;[0 0 0] Get Location for sound and player ref
  (|CallParentFunction)
  (Utilities|FlowControl|Sequence
    (:then_0
      (Variables|Default|SetDoorSoundLocation (Transformation|GetWorldLocation (Variables|Default|GetStaticMesh))))
    (:then_1
      (bind _asbp_character_base (Utilities|Casting|CastTo (Game|GetPlayerCharacter 0)))
      (Variables|Default|SetPlayerRef 0 _asbp_character_base))))

(event EventOnInteract
  ;[0 0 0] Door Logic
  (if (Variables|DoorSettings|Custom|GetLocked)
    (bind _haskey (CallFunction|LookforKey (Variables|/Game/PuzzleSystem/Blueprints/Core/Components/AC_SaveManager.AC_SaveManager_C|GetKeys (CallFunction|GetSaveManager))))
    (if _haskey
      (if (not (Audio|Components|Audio|IsPlaying (Variables|Default|GetTL_Door))) :!label _label
        (if (Variables|DoorSettings|Custom|GetIsClosed?)
          (Variables|DoorSettings|Custom|SetIsClosed? false)
          (CallFunction|DoorOpenSound)
          (bind _alpha (Timeline|TL_Door PlayFromStart)
            (:Update
              (Transformation|SetRelativeRotation (Variables|Default|GetStaticMesh) (Math|Rotator|MakeRotator 0.0 0.0 (Math|Float|Lerp 0.0 (select (Variables|DoorSettings|Custom|GetInvert) -85.0 85.0) _alpha)) false false)))
          (else
            (Variables|DoorSettings|Custom|SetIsClosed? true)
            (CallFunction|DoorCloseSound)
            (Timeline|TL_Door ReverseFromEnd))))
      (else
        (|ForceDoor)))
    (else
      (goto _label))))

(fn ConstructionScript
  (|CallParentFunction)
  (if (Variables|DoorSettings|Custom|GetIsClosed?)
    (Transformation|SetRelativeRotation (Variables|Default|GetStaticMesh) "0, 0, 0" false false)
    (elif (Variables|DoorSettings|Custom|GetInvert)
      (Transformation|SetRelativeRotation (Variables|Default|GetStaticMesh) "0.000000,-85.000000,0.000000" false false)
      (else
        (Transformation|SetRelativeRotation (Variables|Default|GetStaticMesh) "0.000000,85.000000,0.000000" false false)))))

(fn LookforKey
  (params (Keys :type Array%20of%20Integers))
  (bind _array_element (Utilities|Array|ForEachLoopwithBreak Keys :!label _label)
    (:LoopBody
      (if (== _array_element (Variables|DoorSettings|Custom|GetKeyID))
        (LocalVariables|SetDidFindKey true)
        (goto _label Break)))
    (:Completed
      (return (LocalVariables|GetDidFindKey)))))

(event Custom|LockedSequence
  (CallFunction|ForcetoOpen)
  (bind _alpha (Timeline|TL_ForceOpen PlayFromStart)
    (:Update
      (Transformation|SetRelativeRotation (Variables|Default|GetStaticMesh) (Math|Rotator|MakeRotator 0.0 0.0 _alpha) false false))))