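; BP_GhostGear3 is a simple-puzzle actor, a ghost gear whose mesh moves along a timeline-driven path.
; On BeginPlay the Position timeline plays and feeds its PositionUpDown track straight into the static mesh's relative location, without sweep.
; A second timeline for the glow intensity and opacity material parameters is left unconnected and never runs, as is a StartPosition assignment.
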(event EventBeginPlay
  (Utilities|FlowControl|Sequence
    (:then_1
      (bind _position_up_down (Timeline|position Play)
        (:Update
          (Transformation|SetRelativeLocation (Variables|Default|GetStaticMesh) _position_up_down false false))))))

(event Collision|EventActorBeginOverlap
  (params (OtherActor :type Actor%20Object%20Reference)))

(event EventTick
  (params (DeltaSeconds :type Float%20%28single-precision%29)))

(fn ConstructionScript)