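; BP_PickupItem03 is a pickup piece for a simple VR puzzle that must be brought to a placement zone.
; When its box overlaps a BP_PlacementZone, it unhides the first actor tagged RotatableReveal03, reports the piece to BP_SimplePuzzleManager and destroys itself.
; A separate highlight sphere swaps the mesh to a glowing clock material while the VRPawn overlaps it and restores the main material afterwards.
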(event OnComponentBeginOverlap(Box)
  (params (OverlappedComponent :type Primitive%20Component%20Object%20Reference) (OtherActor :type Actor%20Object%20Reference) (OtherComp :type Primitive%20Component%20Object%20Reference) (OtherBodyIndex :type Integer) (bFromSweep :type Boolean) (SweepResult :type Hit%20Result%20Structure%20%28by%20ref%29))
  (Utilities|Casting|CastToBP_PlacementZone OtherActor)
  (bind _outactors (Actor|GetAllActorswithTag "RotatableReveal03"))
  (Rendering|SetActorHiddenInGame (Utilities|Array|Get(acopy) _outactors) false)
  (bind _returnvalue (Actor|GetActorOfClass "/Game/PuzzleSystem/Blueprints/Actors/Simplepuzzle/BP_SimplePuzzleManager.BP_SimplePuzzleManager_C"))
  (bind _asbp_simple_puzzle_manager (Utilities|Casting|CastToBP_SimplePuzzleManager _returnvalue))
  (Default|Pieceplaced _asbp_simple_puzzle_manager)
  (Actor|DestroyActor))

(event OnComponentBeginOverlap(highlightsphere)
  (params (OverlappedComponent :type Primitive%20Component%20Object%20Reference) (OtherActor :type Actor%20Object%20Reference) (OtherComp :type Primitive%20Component%20Object%20Reference) (OtherBodyIndex :type Integer) (bFromSweep :type Boolean) (SweepResult :type Hit%20Result%20Structure%20%28by%20ref%29))
  (Utilities|Casting|CastToVRPawn OtherActor)
  (Rendering|Material|SetMaterial (Variables|Default|GetStaticMesh) 0 "/Game/Assets/MI_Glow_Clock.MI_Glow_Clock"))

(event OnComponentEndOverlap(highlightsphere)
  (params (OverlappedComponent :type Primitive%20Component%20Object%20Reference) (OtherActor :type Actor%20Object%20Reference) (OtherComp :type Primitive%20Component%20Object%20Reference) (OtherBodyIndex :type Integer))
  (Utilities|Casting|CastToVRPawn OtherActor)
  (Rendering|Material|SetMaterial (Variables|Default|GetStaticMesh) 0 "/Game/Assets/MainClock/textures/MI_MainClock.MI_MainClock"))

(event EventBeginPlay)

(event Collision|EventActorBeginOverlap
  (params (OtherActor :type Actor%20Object%20Reference)))

(event EventTick
  (params (DeltaSeconds :type Float%20%28single-precision%29)))

(fn ConstructionScript)