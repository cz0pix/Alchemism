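; BP_GhostGear2 is a translucent ghost gear for a simple puzzle that acts as a visual hint for BP_PickupItem02.
; When that item enters the Hintzone, a timeline animates the mesh materials' glow intensity and opacity parameters.
; When it leaves, the timeline stops and both parameters reset to fixed values.
; A separate Position timeline starts on BeginPlay and drives the mesh's relative location for an up-and-down motion.
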(event OnComponentBeginOverlap(hintzone)
  (params (OverlappedComponent :type Primitive%20Component%20Object%20Reference) (OtherActor :type Actor%20Object%20Reference) (OtherComp :type Primitive%20Component%20Object%20Reference) (OtherBodyIndex :type Integer) (bFromSweep :type Boolean) (SweepResult :type Hit%20Result%20Structure%20%28by%20ref%29))
  (Utilities|Casting|CastToBP_PickupItem02 OtherActor)
  (bind (_direction _glow_intensity _opacity_amount) (Timeline|Timeline Play)
    (:Update
      (Utilities|FlowControl|Sequence
        (:then_0
          (Rendering|Material|SetScalarParameterValueonMaterials (Variables|Default|GetStaticMesh) "glow intensity" _glow_intensity))
        (:then_1
          (Rendering|Material|SetScalarParameterValueonMaterials (Variables|Default|GetStaticMesh) "opacity amount" _opacity_amount))))))

(event OnComponentEndOverlap(hintzone)
  (params (OverlappedComponent :type Primitive%20Component%20Object%20Reference) (OtherActor :type Actor%20Object%20Reference) (OtherComp :type Primitive%20Component%20Object%20Reference) (OtherBodyIndex :type Integer))
  (Utilities|Casting|CastToBP_PickupItem02 OtherActor)
  (Utilities|FlowControl|Sequence
    (:then_0
      (bind (_direction _glow_intensity _opacity_amount) (Timeline|Timeline Stop)
        (:Update
          (Utilities|FlowControl|Sequence
            (:then_0
              (Rendering|Material|SetScalarParameterValueonMaterials (Variables|Default|GetStaticMesh) "glow intensity" _glow_intensity))
            (:then_1
              (Rendering|Material|SetScalarParameterValueonMaterials (Variables|Default|GetStaticMesh) "opacity amount" _opacity_amount))))))
    (:then_1
      (Rendering|Material|SetScalarParameterValueonMaterials (Variables|Default|GetStaticMesh) "glow intensity" 0.6)
      (Rendering|Material|SetScalarParameterValueonMaterials (Variables|Default|GetStaticMesh) "opacity amount" 0.2))))

(event EventBeginPlay
  (Utilities|FlowControl|Sequence
    (:then_1
      (bind _position_up_down (Timeline|position Play)
        (:Update
          (Transformation|SetRelativeLocation (Variables|Default|GetStaticMesh) _position_up_down false false))))))

(event Collision|EventActorBeginOverlap
  (params (OtherActor :type Actor%20Object%20Reference)))

(event EventTick
  (params (DeltaSeconds :type Float%20%28single-precision%29)))

(fn ConstructionScript)