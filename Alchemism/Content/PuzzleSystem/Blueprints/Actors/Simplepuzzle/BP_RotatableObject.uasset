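; Puzzle actor whose static mesh rotates when something overlaps its interaction zone.
; A separate Box overlap plays a timeline that moves a Cube along Z and turns the mesh again on every update.
; A Rotateobject event prints a debug message and yaws the whole actor.
; Player input is enabled, but the rotate input action is empty, and the CanRotate gate and VR rotation nodes are disconnected.
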(event OnComponentBeginOverlap(interactionzone)
  (params (OverlappedComponent :type Primitive%20Component%20Object%20Reference) (OtherActor :type Actor%20Object%20Reference) (OtherComp :type Primitive%20Component%20Object%20Reference) (OtherBodyIndex :type Integer) (bFromSweep :type Boolean) (SweepResult :type Hit%20Result%20Structure%20%28by%20ref%29))
  (Transformation|AddLocalRotation (Variables|Default|GetStaticMesh) "0.000000,0.000000,90.000000" false false))

(event OnComponentEndOverlap(interactionzone)
  (params (OverlappedComponent :type Primitive%20Component%20Object%20Reference) (OtherActor :type Actor%20Object%20Reference) (OtherComp :type Primitive%20Component%20Object%20Reference) (OtherBodyIndex :type Integer))
  (Variables|Default|SetCanRotate false))

(event OnComponentBeginOverlap(Box)
  (params (OverlappedComponent :type Primitive%20Component%20Object%20Reference) (OtherActor :type Actor%20Object%20Reference) (OtherComp :type Primitive%20Component%20Object%20Reference) (OtherBodyIndex :type Integer) (bFromSweep :type Boolean) (SweepResult :type Hit%20Result%20Structure%20%28by%20ref%29))
  (bind _newtrack_0 (Timeline|Timeline Play)
    (:Update
      (Transformation|SetRelativeLocationAndRotation (Variables|Default|GetCube) (Math|Vector|MakeVector 0.0 0.0 _newtrack_0) "0, 0, 0" false false)
      (Transformation|AddLocalRotation (Variables|Default|GetStaticMesh) "0.000000,0.000000,90.000000" false false))))

(event Custom|Rotateobject
  (Development|PrintString "rotate")
  (Transformation|AddActorLocalRotation (Math|Rotator|MakeRotator 0.0 0.0 15.0) false false))

(event Input|EnhancedActionEvents|EnhancedInputActionIA_RotatePuzzle
  (params (ActionValue :type Boolean) (ElapsedSeconds :type Float%20%28double-precision%29) (TriggeredSeconds :type Float%20%28double-precision%29) (InputAction :type Input%20Action%20Object%20Reference :default "/Game/VRTemplate/Input/Actions/IA_RotatePuzzle.IA_RotatePuzzle")))

(event EventBeginPlay
  (Input|EnableInput (Game|GetPlayerController 0)))

(event Collision|EventActorBeginOverlap
  (params (OtherActor :type Actor%20Object%20Reference)))

(event EventTick
  (params (DeltaSeconds :type Float%20%28single-precision%29)))

(event Input|GamepadEvents|GamepadRightTrigger
  (params (Key :type Key%20Structure :default "None")))

(fn ConstructionScript)