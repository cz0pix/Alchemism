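; BP_SimplePuzzleManager is the puzzle manager that counts placed pieces and plays the completion sequence ending the puzzle.
; Each Pieceplaced call increments a counter, and at four it rotates four rotatable objects found by class, swapping each to a glow material after a delay.
; Delayed branches then hide the clock face, reveal a Niagara actor and later add the end screen widget to the viewport.
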(event Custom|Pieceplaced
  (bind _result (Math|Integer|IncrementInt (Variables|Default|GetPlacedPieces))
    (:%20%20
      (bind _output_get (Variables|Default|SetPlacedPieces _result))
      (Development|PrintString "AAAA")
      (if (>= _output_get 4)
        (Development|PrintString "xxxxxxxxxxxxxxxxxxxxxxxxxxxxxxxxxxxxxxxxxxxxxxx")
        (Utilities|FlowControl|Sequence
          (:then_0
            (bind _outactors (Actor|GetAllActorsOfClass "/Game/PuzzleSystem/Blueprints/Actors/Simplepuzzle/BP_RotatableObject01.BP_RotatableObject01_C"))
            (Default|PlayRotateAnimation (Utilities|Array|Get(acopy) _outactors))
            (Utilities|FlowControl|Delay 2.0)
            (Rendering|Material|SetMaterial (Variables|/Game/PuzzleSystem/Blueprints/Actors/Simplepuzzle/BP_RotatableObject01.BP_RotatableObject01_C|GetStaticMesh (Utilities|Array|Get(acopy) _outactors)) 0 "/Game/Assets/M_Glow2_AssetMaterial2.M_Glow2_AssetMaterial2"))
          (:then_1
            (bind _outactors_2 (Actor|GetAllActorsOfClass "/Game/PuzzleSystem/Blueprints/Actors/Simplepuzzle/BP_RotatableObject02.BP_RotatableObject02_C"))
            (Default|PlayRotateAnimation (Utilities|Array|Get(acopy) _outactors_2))
            (Utilities|FlowControl|Delay 2.0)
            (Rendering|Material|SetMaterial (Variables|/Game/PuzzleSystem/Blueprints/Actors/Simplepuzzle/BP_RotatableObject02.BP_RotatableObject02_C|GetStaticMesh (Utilities|Array|Get(acopy) _outactors_2)) 0 "/Game/Assets/M_Glow2_AssetMaterial2.M_Glow2_AssetMaterial2"))
          (:then_2
            (bind _outactors_3 (Actor|GetAllActorsOfClass "/Game/PuzzleSystem/Blueprints/Actors/Simplepuzzle/BP_RotatableObject03.BP_RotatableObject03_C"))
            (Default|PlayRotateAnimation (Utilities|Array|Get(acopy) _outactors_3))
            (Utilities|FlowControl|Delay 2.0)
            (Rendering|Material|SetMaterial (Variables|/Game/PuzzleSystem/Blueprints/Actors/Simplepuzzle/BP_RotatableObject03.BP_RotatableObject03_C|GetStaticMesh (Utilities|Array|Get(acopy) _outactors_3)) 0 "/Game/Assets/M_Glow2_AssetMaterial2.M_Glow2_AssetMaterial2"))
          (:then_3
            (bind _outactors_4 (Actor|GetAllActorsOfClass "/Game/PuzzleSystem/Blueprints/Actors/Simplepuzzle/BP_RotatableObject04.BP_RotatableObject04_C"))
            (Default|PlayRotateAnimation (Utilities|Array|Get(acopy) _outactors_4))
            (Utilities|FlowControl|Delay 2.0)
            (Rendering|Material|SetMaterial (Variables|/Game/PuzzleSystem/Blueprints/Actors/Simplepuzzle/BP_RotatableObject04.BP_RotatableObject04_C|GetStaticMesh (Utilities|Array|Get(acopy) _outactors_4)) 0 "/Game/Assets/M_Glow2_AssetMaterial2.M_Glow2_AssetMaterial2"))
          (:then_4
            (Utilities|FlowControl|Delay 2.0)
            (bind _outactors_5 (Actor|GetAllActorsOfClass "/Game/PuzzleSystem/Blueprints/Actors/Simplepuzzle/Bp_ClockFace.Bp_ClockFace_C"))
            (Rendering|SetActorHiddenInGame (Utilities|Array|Get(acopy) _outactors_5) true))
          (:then_5
            (Utilities|FlowControl|Delay 2.0)
            (bind _outactors_6 (Actor|GetAllActorsOfClass "/Game/PuzzleSystem/Blueprints/Actors/Simplepuzzle/BP_Niagara.BP_Niagara_C"))
            (Rendering|SetActorHiddenInGame (Utilities|Array|Get(acopy) _outactors_6) false)
            (Utilities|FlowControl|Delay 7.0)
            (bind _returnvalue (UserInterface|CreateWidget "/Game/Cutscene/WBP_EndScreen.WBP_EndScreen_C"))
            (UserInterface|Viewport|AddtoViewport _returnvalue 0)))))))

(event EventBeginPlay)

(event Collision|EventActorBeginOverlap
  (params (OtherActor :type Actor%20Object%20Reference)))

(event EventTick
  (params (DeltaSeconds :type Float%20%28single-precision%29)))

(fn ConstructionScript)