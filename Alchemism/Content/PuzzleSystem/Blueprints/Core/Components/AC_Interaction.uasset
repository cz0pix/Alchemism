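; Player interaction component for a puzzle system that detects, outlines, uses and inspects actors.
; A looping timer line-traces from the character's camera, tracking and outlining hit actors that implement BPI_BFInteraction.
; Inspection hides the actor, spawns a rotatable copy far off in the world and shows a widget with readable text.
; InteractActor fetches the target's data, but its switch between Interact and Inspect is unconnected.
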(event Custom|InspectionRotation
  (params (Direction :type Vector%202D%20Structure))
  (|SetInspectionRotation Direction))

(event EventBeginPlay
  (Utilities|Time|SetTimerbyFunctionName 0 "TraceActor" 0.1 true))

(fn TraceActor
  (bind (_start _end) (Utilities|TraceConditions)
    (:Output
      (bind (_outhit _returnvalue) (Collision|LineTraceByChannel _start _end "TraceTypeQuery1" false 0 (Variables|Default|GetDraw%20Debug%20Type)))
      (if _returnvalue
        (Utilities|IsValid (.HitActor (Collision|BreakHitResult _outhit))
          (:Is%20Valid
            (if (Utilities|DoesObjectImplementInterface (.HitActor (Collision|BreakHitResult _outhit)) "/Game/PuzzleSystem/Blueprints/Core/Interfaces/BPI_BFInteraction.BPI_BFInteraction_C")
              (bind _output_get (Variables|Default|SetInteractionActor (.HitActor (Collision|BreakHitResult _outhit))))
              (CallFunction|CustomOutline _output_get true)
              (else
                (Core|ResetInteract :!label _label))))
          (:Is%20Not%20Valid
            (goto _label)))
        (else
          (goto _label))))))

(fn InteractActor
  (Class|BPIBFInteraction|GetData(Message) (Variables|Default|GetInteractionActor)))

(fn SpawnInspectionActor
  (bind (_meshsettings _inspectionsettings) (Utilities|Struct|Break))
  (bind _returnvalue (Game|SpawnActorfromClass 0 (Math|Transform|MakeTransform "100000000.000000,0.000000,0.000000") "Undefined" "MultiplyWithRoot" 0 0))
  (Variables|Default|SetInspectionActor 0 _returnvalue)
  (CallFunction|OnInspectCreated _returnvalue (.staticmesh _meshsettings) (.offset _inspectionsettings) (.distance _inspectionsettings) (.rotation _inspectionsettings)))

(fn StopInspect
  (CallFunction|SetActive (.InspectWidgetRef (Variables|Default|GetInspectWidgetRef)) true)
  (CallFunction|UpdateInputMapping)
  (Utilities|IsValid (.InspectionActor (Variables|Default|GetInspectionActor))
    (:Is%20Valid
      (Actor|DestroyActor (.InspectionActor (Variables|Default|GetInspectionActor)))
      (Rendering|SetActorHiddenInGame (Variables|Default|GetInteractionActor) false)
      (Variables|Default|SetInspectionActor 0)
      (Variables|Default|SetInspectWidgetRef 0))))

(fn ResetInteract
  (Variables|Default|GetInteractionActor
    (:then
      (CallFunction|CustomOutline (Variables|Default|GetInteractionActor) false)
      (Variables|Default|SetInteractionActor 0))
    (:else)))

(fn DisplayPages
  (bind _inspectwidgetref (Variables|Default|GetInspectWidgetRef))
  (Utilities|IsValid (.InspectWidgetRef (Variables|Default|GetInspectWidgetRef))
    (:Is%20Valid
      (if (Variables|Default|GetIsreading (.InspectWidgetRef (Variables|Default|GetInspectWidgetRef)))
        (CallFunction|DisplayText _inspectwidgetref true)
        (Inspection|ChangeReadingState)
        (else
          (CallFunction|DisplayText _inspectwidgetref false)
          (Inspection|ChangeReadingState))))))

(fn ChangeReadingState
  (Variables|Default|SetIsReading (Variables|Default|GetIsreading (.InspectWidgetRef (Variables|Default|GetInspectWidgetRef)))))