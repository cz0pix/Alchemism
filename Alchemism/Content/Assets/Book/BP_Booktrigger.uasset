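; BP_Booktrigger is a trigger volume that animates a referenced book when the VR pawn enters its zone.
; Overlap begin plays the book's geometry cache at normal speed.
; Overlap end prints a debug string, stops the cache running and resets its start time offset to zero.
; Reverse-playback nodes are present but unconnected.
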(event OnComponentBeginOverlap(triggerzone)
  (params (OverlappedComponent :type Primitive%20Component%20Object%20Reference) (OtherActor :type Actor%20Object%20Reference) (OtherComp :type Primitive%20Component%20Object%20Reference) (OtherBodyIndex :type Integer) (bFromSweep :type Boolean) (SweepResult :type Hit%20Result%20Structure%20%28by%20ref%29))
  (bind _bookref (Variables|Default|GetBookref))
  (bind _geometrycachecomponent (Variables|/Script/GeometryCache.GeometryCacheActor|GetGeometryCacheComponent _bookref))
  (Utilities|Casting|CastToVRPawn OtherActor)
  (Class|GeometryCacheComponent|SetPlaybackSpeed _geometrycachecomponent 1.0)
  (Audio|Components|Audio|Play _geometrycachecomponent))

(event OnComponentEndOverlap(triggerzone)
  (params (OverlappedComponent :type Primitive%20Component%20Object%20Reference) (OtherActor :type Actor%20Object%20Reference) (OtherComp :type Primitive%20Component%20Object%20Reference) (OtherBodyIndex :type Integer))
  (bind _bookref (Variables|Default|GetBookref))
  (bind _geometrycachecomponent (Variables|/Script/GeometryCache.GeometryCacheActor|GetGeometryCacheComponent _bookref))
  (Utilities|Casting|CastToVRPawn OtherActor)
  (Development|PrintString "XXXXXXXXXXXXXXXXXXXXXXXXXXXXXXXXXXXXXXXXXXXXXXXXXXXXXXXXXX")
  (Variables|/Script/GeometryCache.GeometryCacheComponent|SetbRunning _geometrycachecomponent false)
  (Class|GeometryCacheComponent|SetStartTimeOffset _geometrycachecomponent 0.0))

(event EventBeginPlay)

(event Collision|EventActorBeginOverlap
  (params (OtherActor :type Actor%20Object%20Reference)))

(event EventTick
  (params (DeltaSeconds :type Float%20%28single-precision%29)))

(fn ConstructionScript)