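; Rat actor whose skeletal mesh runs along a spline path on a repeating loop, starting at BeginPlay.
; A timeline, with play rate set by Speed, maps its track to distance along the spline and sets the mesh's world location and rotation, with yaw offset by -90 degrees.
; When a run finishes, it waits a random few seconds before restarting from the spline's start.
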(event Custom|Ride
  (Components|Timeline|SetPlayRate (Variables|Default|GetRideTimeline) (Variables|Default|GetSpeed))
  (bind _ridetrack (Timeline|RideTimeline PlayFromStart)
    (:Update
      (Transformation|SetWorldLocationAndRotation (Variables|Default|GetSKM_rat) (.location (Spline|GetTransformatDistanceAlongSpline (Variables|Default|GetSpline) (Math|Float|Lerp 0.0 (Spline|GetSplineLength (Variables|Default|GetSpline)) _ridetrack) "World" false)) (Math|Rotator|MakeRotator (.roll (.rotation (Spline|GetTransformatDistanceAlongSpline (Variables|Default|GetSpline) (Math|Float|Lerp 0.0 (Spline|GetSplineLength (Variables|Default|GetSpline)) _ridetrack) "World" false))) (.pitch (.rotation (Spline|GetTransformatDistanceAlongSpline (Variables|Default|GetSpline) (Math|Float|Lerp 0.0 (Spline|GetSplineLength (Variables|Default|GetSpline)) _ridetrack) "World" false))) (- (.yaw (.rotation (Spline|GetTransformatDistanceAlongSpline (Variables|Default|GetSpline) (Math|Float|Lerp 0.0 (Spline|GetSplineLength (Variables|Default|GetSpline)) _ridetrack) "World" false))) 9e+01)) false false))
    (:Finished
      (Utilities|FlowControl|Delay (Math|Random|RandomFloatinRange 3.0 1e+01))
      (CallFunction|Ride))))

(event EventBeginPlay
  (CallFunction|Ride))

(fn ConstructionScript)